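; BP_Controller is a player controller for a game with card effects, creating the BP_InGame HUD widget and routing left-click input.
; A DoubleClickCheck macro counts clicks, reset by a short retriggerable delay, to fire first or second press and release events while CardEffectTargets is empty.
; When targets exist, releasing the button calls OnClickTarget instead.
; Debug helpers print the target-empty state every tick and toggle slow motion on key 1.
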(event Input|EnhancedActionEvents|EnhancedInputActionLeftMouseButton
  (params (ActionValue :type Boolean) (ElapsedSeconds :type Float%20%28double-precision%29) (TriggeredSeconds :type Float%20%28double-precision%29) (InputAction :type Input%20Action%20Object%20Reference :default "/Game/Input/LeftMouseButton.LeftMouseButton"))
  (bind _cardeffecttargets (Variables|Default|GetCardEffectTargets))
  (:Started
    (if (Utilities|Array|IsEmpty _cardeffecttargets)
      (Utilities|DoubleClickCheck
        (:SingleClick
          (Class|GameController|OnFirstPress))
        (:DoubleClick
          (Class|GameController|OnSecondPress)))))
  (:Completed
    (if (Utilities|Array|IsEmpty _cardeffecttargets)
      (Utilities|DoubleClickCheck
        (:SingleClick
          (Class|GameController|OnFirstRelease))
        (:DoubleClick
          (Class|GameController|OnSecondRelease)))
      (else
        (Class|GameController|OnClickTarget)))))

(event EventBeginPlay
  (bind _returnvalue (UserInterface|CreateWidget "/Game/UMG/BP_InGame.BP_InGame_C" self))
  (Utilities|IsValid _returnvalue
    (:Is%20Valid
      (UserInterface|Viewport|AddtoViewport _returnvalue 0))))

(event EventTick
  (params (DeltaSeconds :type Float%20%28single-precision%29))
  (Development|PrintString (Utilities|String|ToString(Boolean) (Utilities|Array|IsEmpty (Variables|Default|GetCardEffectTargets))) true true "(R=0.000000,G=0.660000,B=1.000000,A=1.000000)" 0.0))

(event Input|KeyboardEvents|1
  (params (Key :type Key%20Structure :default "None"))
  (:Pressed
    (Utilities|FlowControl|FlipFlop
      (:A
        (Utilities|Time|SetGlobalTimeDilation 0.1))
      (:B
        (Utilities|Time|SetGlobalTimeDilation 1.0)))))

(fn ConstructionScript)