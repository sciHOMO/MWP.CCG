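; Card actor for a card game that handles the visual side of drawing, entry, attack, damage, activation and casting.
; Each animation event calls its parent, then spawns a short-lived Level Sequence player, rebinding the card to bindings often chosen by player, team or position.
; Entry can also trigger a UI montage, and attack end plays a camera sequence on both players' cameras.
; Cursor hover toggles overlap messages, and card updates refresh the AP:HP text.
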(event OnBeginCursorOver(CardCollision)
  (params (TouchedComponent :type Primitive%20Component%20Object%20Reference))
  (Class|Interact|StartOverlap(Message) self))

(event OnBeginCursorOver(PawnCollision)
  (params (TouchedComponent :type Primitive%20Component%20Object%20Reference))
  (Class|Interact|StartOverlap(Message) self))

(event OnEndCursorOver(CardCollision)
  (params (TouchedComponent :type Primitive%20Component%20Object%20Reference))
  (Class|Interact|StopOverlap(Message) self))

(event OnEndCursorOver(PawnCollision)
  (params (TouchedComponent :type Primitive%20Component%20Object%20Reference))
  (Class|Interact|StopOverlap(Message) self))

(event EventPlayDrawAnim
  (params (Event :type Order%20Update%20Event%20Structure%20%28by%20ref%29))
  (|CallParentFunction Event)
  (bind (_outactor _returnvalue) (Sequencer|Player|CreateLevelSequencePlayer "/Game/Level/Sequence/Draw.Draw" (Utilities|Struct|MakeMovieSceneSequencePlaybackSettings false "(Value=0)" "(TickIntervalSeconds=0.000000,EvaluationBudgetMicroseconds=0.000000,bTickWhenPaused=False,bAllowRounding=True)" 1.3 0.0 false false false false false false "ForceKeepState")))
  (Class|LevelSequenceActor|AddBinding _outactor (Utilities|Select :Index (Utilities|Struct|BreakCardInfo (Variables|Default|GetCardInfo)) :Option%200 (Utilities|Select :Index (Variables|Default|GetTeam) :PlaceHolder "" :Owner (|GetSequenceBinding) :Opponent (|GetSequenceBinding)) :Option%201 (Utilities|Select :Index (Variables|Default|GetTeam) :PlaceHolder "" :Owner (|GetSequenceBinding) :Opponent (|GetSequenceBinding))) self false)
  (EventDispatchers|BindEventtoOnFinished _returnvalue (EventDispatchers|CreateEvent :!event DrawAnimEnd))
  (Sequencer|Player|Play _returnvalue :!class /Script/MovieScene.MovieSceneSequencePlayer)
  (Actor|SetLifeSpan _outactor 3.0))

(event EventPlayEntryAnim
  (params (Event :type Order%20Update%20Event%20Structure%20%28by%20ref%29))
  (|CallParentFunction Event)
  (bind (_outactor _returnvalue) (Sequencer|Player|CreateLevelSequencePlayer "/Game/Level/Sequence/Entry_1.Entry_1" (Utilities|Struct|MakeMovieSceneSequencePlaybackSettings false "(Value=0)" "(TickIntervalSeconds=0.000000,EvaluationBudgetMicroseconds=0.000000,bTickWhenPaused=False,bAllowRounding=True)" 1.0 0.0 false false false false false false "ForceKeepState")))
  (Class|LevelSequenceActor|AddBinding _outactor (Utilities|Select :Index (Utilities|Struct|BreakCardInfo (Variables|Default|GetCardInfo)) :Option%200 (|GetSequenceBinding) :Option%201 (|GetSequenceBinding)) self true)
  (Sequencer|Player|Play _returnvalue :!class /Script/MovieScene.MovieSceneSequencePlayer)
  (Actor|SetLifeSpan _outactor 3.0))

(event EventPlayEntryAnimC
  (params (Event :type Order%20Update%20Event%20Structure%20%28by%20ref%29))
  (bind _positioninfo (Utilities|Struct|BreakOrderUpdateEvent Event))
  (bind _output (Utilities|Array|Get(acopy) _positioninfo 1))
  (bind (_x _y) (Utilities|Struct|BreakIntPoint _output))
  (|CallParentFunction Event)
  (CallFunction|ShowMontage)
  (Utilities|FlowControl|Delay 0.5)
  (bind (_outactor _returnvalue) (Sequencer|Player|CreateLevelSequencePlayer "/Game/Level/Sequence/Entry_2.Entry_2" (Utilities|Struct|MakeMovieSceneSequencePlaybackSettings false "(Value=0)" "(TickIntervalSeconds=0.000000,EvaluationBudgetMicroseconds=0.000000,bTickWhenPaused=False,bAllowRounding=True)" 1.2)))
  (Class|LevelSequenceActor|AddBinding _outactor (Utilities|Select :Index _y :Option%200 (Utilities|Select :Index _x :Option%200 (|GetSequenceBinding) :Option%201 (|GetSequenceBinding)) :Option%201 (Utilities|Select :Index _x :Option%200 (|GetSequenceBinding) :Option%201 (|GetSequenceBinding)) :Option%202 (Utilities|Select :Index _x :Option%200 (|GetSequenceBinding) :Option%201 (|GetSequenceBinding)) :Option%203 (Utilities|Select :Index _x :Option%200 (|GetSequenceBinding) :Option%201 (|GetSequenceBinding))) self true)
  (EventDispatchers|BindEventtoOnFinished _returnvalue (EventDispatchers|CreateEvent :!event EntryAnimEnd))
  (Sequencer|Player|Play _returnvalue :!class /Script/MovieScene.MovieSceneSequencePlayer)
  (Actor|SetLifeSpan _outactor 3.0))

(event EventPlayAttackAnim
  (params (Event :type Order%20Update%20Event%20Structure%20%28by%20ref%29))
  (|CallParentFunction Event)
  (bind (_outactor _returnvalue) (Sequencer|Player|CreateLevelSequencePlayer "/Game/Level/Sequence/Attack.Attack"))
  (Class|LevelSequenceActor|AddBinding _outactor (|GetSequenceBinding) self false)
  (EventDispatchers|BindEventtoOnFinished _returnvalue (EventDispatchers|CreateEvent :!event AttackAnimEnd))
  (Sequencer|Player|Play _returnvalue :!class /Script/MovieScene.MovieSceneSequencePlayer)
  (Actor|SetLifeSpan _outactor 3.0))

(event EventPlayDamageAnim
  (params (Event :type Order%20Update%20Event%20Structure%20%28by%20ref%29))
  (|CallParentFunction Event)
  (bind (_outactor _returnvalue) (Sequencer|Player|CreateLevelSequencePlayer "/Game/Level/Sequence/Damage.Damage"))
  (Class|LevelSequenceActor|AddBinding _outactor (|GetSequenceBinding) self false)
  (EventDispatchers|BindEventtoOnFinished _returnvalue (EventDispatchers|CreateEvent :!event DamageAnimEnd))
  (Sequencer|Player|Play _returnvalue :!class /Script/MovieScene.MovieSceneSequencePlayer)
  (Actor|SetLifeSpan _outactor 3.0))

(event EventPlayActivateAnim
  (params (Event :type Order%20Update%20Event%20Structure%20%28by%20ref%29))
  (|CallParentFunction Event)
  (bind (_outactor _returnvalue) (Sequencer|Player|CreateLevelSequencePlayer "/Game/Level/Sequence/Activate.Activate"))
  (Class|LevelSequenceActor|AddBinding _outactor (select (>= (.z (Variables|/Script/Engine.SceneComponent|GetRelativeLocation (Variables|Default|GetPawnMesh))) 25.0) (|GetSequenceBinding) (|GetSequenceBinding)) self false)
  (EventDispatchers|BindEventtoOnFinished _returnvalue (EventDispatchers|CreateEvent :!event ActivateAnimEnd))
  (Sequencer|Player|Play _returnvalue :!class /Script/MovieScene.MovieSceneSequencePlayer)
  (Actor|SetLifeSpan _outactor 3.0))

(event EventPlayCastAnim
  (params (Event :type Order%20Update%20Event%20Structure%20%28by%20ref%29))
  (|CallParentFunction Event)
  (bind (_outactor _returnvalue) (Sequencer|Player|CreateLevelSequencePlayer "/Game/Level/Sequence/Cast.Cast" (Utilities|Struct|MakeMovieSceneSequencePlaybackSettings false "(Value=0)" "(TickIntervalSeconds=0.000000,EvaluationBudgetMicroseconds=0.000000,bTickWhenPaused=False,bAllowRounding=True)" 1.0 0.0 false false false false false false "ForceKeepState")))
  (Class|LevelSequenceActor|AddBinding _outactor (Utilities|Select :Index (Utilities|Struct|BreakCardInfo (Variables|Default|GetCardInfo)) :Option%200 (Utilities|Select :Index (Variables|Default|GetTeam) :PlaceHolder "" :Owner (|GetSequenceBinding) :Opponent (|GetSequenceBinding)) :Option%201 (Utilities|Select :Index (Variables|Default|GetTeam) :PlaceHolder "" :Owner (|GetSequenceBinding) :Opponent (|GetSequenceBinding))) self true)
  (EventDispatchers|BindEventtoOnFinished _returnvalue (EventDispatchers|CreateEvent :!event CastAnimEnd))
  (Sequencer|Player|Play _returnvalue :!class /Script/MovieScene.MovieSceneSequencePlayer)
  (Actor|SetLifeSpan _outactor 3.0))

(fn ConstructionScript)

(fn ShowMontage
  (bind _foundwidgets (Class|WidgetBlueprintLibrary|GetAllWidgetswithInterface "/Script/MirrorRealmProtocol.ToUMG" false))
  (Class|ToUMG|ShowMontage(Message) (Utilities|Array|Get(acopy) _foundwidgets) (Utilities|Struct|BreakCardInfo (Variables|Default|GetCardInfo))))

(fn AttackAnimEnd
  (|CallParentFunction)
  (Utilities|FlowControl|Sequence
    (:then_0
      (bind _outactors (Actor|GetAllActorsOfClasswithTag "/Script/Engine.CameraActor" "Player_0"))
      (bind (_outactor _returnvalue) (Sequencer|Player|CreateLevelSequencePlayer "/Game/Level/Sequence/AttackCamera.AttackCamera"))
      (Class|LevelSequenceActor|AddBinding _outactor (|GetSequenceBinding) (Utilities|Array|Get(acopy) _outactors) true)
      (Sequencer|Player|Play _returnvalue :!class /Script/MovieScene.MovieSceneSequencePlayer)
      (Actor|SetLifeSpan _outactor 3.0))
    (:then_1
      (bind _outactors_2 (Actor|GetAllActorsOfClasswithTag "/Script/Engine.CameraActor" "Player_1"))
      (bind (_outactor_2 _returnvalue_2) (Sequencer|Player|CreateLevelSequencePlayer "/Game/Level/Sequence/AttackCamera.AttackCamera"))
      (Class|LevelSequenceActor|AddBinding _outactor_2 (|GetSequenceBinding) (Utilities|Array|Get(acopy) _outactors_2) true)
      (Sequencer|Player|Play _returnvalue_2 :!class /Script/MovieScene.MovieSceneSequencePlayer)
      (Actor|SetLifeSpan _outactor_2 3.0))))

(fn UpdateCardInfo
  (params (CI :type Card%20Info%20Structure%20%28by%20ref%29))
  (bind (_cardinstid _cardid _cost _realcost _name _cardtype _cardattribute _cardrace _cardeffects _cardspecs _ap _realap _hp _realhp) (Utilities|Struct|BreakCardInfo CI))
  (bind _returnvalue (Utilities|String|ToString(Integer) _realhp))
  (bind _returnvalue_2 (Utilities|String|ToString(Integer) _realap))
  (bind _returnvalue_3 (Utilities|String|Append _returnvalue_2 " : " _returnvalue))
  (Rendering|Components|TextRender|SetText (Variables|Default|GetTextRender) (Class|KismetTextLibrary|MakeInvariantText _returnvalue_3))
  (Development|PrintString (Utilities|String|Append (Utilities|String|ToString(Integer) _cardinstid) " Update :" _returnvalue_3) true true "(R=0.000000,G=0.660000,B=1.000000,A=1.000000)" 1e+02))